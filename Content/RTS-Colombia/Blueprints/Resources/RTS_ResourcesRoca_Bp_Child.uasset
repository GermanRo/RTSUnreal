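; Rock resource child Blueprint for an RTS, where harvester units gather on entering its ResourceEntry component.
; An overlapping RTS_HarvesterUnit has its harvest triggered after a fixed delay, and leaving before its inventory is full triggers an early harvest end.
; Despite the rock name, both calls use the harvester's Maiz (corn) functions, and debug strings print along the way.
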(event `self.ResourceEntry.OnComponentBeginOverlap`
  (params (OverlappedComponent :type "PrimitiveComponent Object Reference") (OtherActor :type "Actor Object Reference") (OtherComp :type "PrimitiveComponent Object Reference") (OtherBodyIndex :type Integer) (bFromSweep :type Boolean) (SweepResult :type "HitResult Structure (by ref)"))
  (bind _asrts_harvester_unit (cast `/Game/RTS-Colombia/Unidades/RTS_HarvesterUnit` OtherActor))
  (`KismetSystemLibrary.PrintString` "maizando")
  (`KismetSystemLibrary.Delay` 5.0)
  (`KismetSystemLibrary.PrintString` "voy a empezar")
  (`/Game/RTS-Colombia/Unidades/RTS_UnidadMaster.HarvestTriggerMaiz` _asrts_harvester_unit))

(event `self.ResourceEntry.OnComponentEndOverlap`
  (params (OverlappedComponent :type "PrimitiveComponent Object Reference") (OtherActor :type "Actor Object Reference") (OtherComp :type "PrimitiveComponent Object Reference") (OtherBodyIndex :type Integer))
  (bind _asrts_harvester_unit (cast `/Game/RTS-Colombia/Unidades/RTS_HarvesterUnit` OtherActor))
  (if (not (`/Game/RTS-Colombia/Unidades/RTS_HarvesterUnit.IsInventoryFull` _asrts_harvester_unit))
    (`KismetSystemLibrary.PrintString` "sali")
    (`/Game/RTS-Colombia/Unidades/RTS_UnidadMaster.EarlyHarvestEndMaiz` _asrts_harvester_unit)))

(fn `UserConstructionScript`
  (`parent.UserConstructionScript`))