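; Resource spawn volume for the RTS that scatters a configured resource class at random points within its bounds.
; Each attempt runs a box trace on Visibility and spawns only where it hits Landscape.
; Spawning can run at BeginPlay and on a looping timer that skips while paused and stops at a maximum count of attempts.
; RespawnTime follows game speed, a custom value or both, recalculated every Tick, but the timer takes it only at BeginPlay.
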(event `self.ReceiveBeginPlay`
  (`|ExecutionSequence`
    (:`then_0`
      (`self.ReferencesCastMacro`))
    (:`then_1`
      (add `/Game/RTS-Colombia/Blueprints/GameSettings/RTS_GameState_BP.GameSpeedControl` (`self.GameStateRef`) (`|CreateDelegate` :!event `GetGameSpeed`))
      (bind _gamespeed (`/Game/RTS-Colombia/Blueprints/GameSettings/RTS_GameState_BP.GetGameSpeed` (`self.GameStateRef`)))
      (set `self.GameSpeed` _gamespeed)
      (`self.SetRespawnTimer`))
    (:`then_2`
      (if (`self.InSpawnOnBeginPlay`)
        (`self.SpawnResource` (`self.ResourceRef`) (`self.NumReosurcesSpawn`))
        (set `self.TotalNumberSpawned` (+ (`self.NumReosurcesSpawn`) (`self.TotalNumberSpawned`))))
      (if (`self.IsSpwanedTimer`)
        (`KismetSystemLibrary.K2_SetTimerDelegate` (`|CreateDelegate` :!event `SpawnResourcesOntimer`) (`self.RespawnTime`) true)))))

(event `GetGameSpeed`
  (params (GameSpeed :type "Float (double-precision)"))
  (set `self.GameSpeed` GameSpeed))

(event `self.ReceiveTick`
  (params (DeltaSeconds :type "Float (single-precision)"))
  (`self.SetRespawnTimer`))

(event `SpawnResourcesOntimer`
  (if (`/Game/RTS-Colombia/Blueprints/Widgets/GameTime_HUD.Ispause` (`/Game/RTS-Colombia/Blueprints/Player/RTS_PlayerController_BP.HUDGameTimeRef` (`self.MyPlayerControllerRef`)))
    _
    (elif (and (`self.IsSpwanedTimer`) (< (`self.TotalNumberSpawned`) (`self.MaxResourcesSpawned`)))
      (`self.SpawnResource` (`self.ResourceRef`) (`self.NumReosurcesSpawn`))
      (set `self.TotalNumberSpawned` (+ (`self.NumReosurcesSpawn`) (`self.TotalNumberSpawned`))))))

(fn `SetRespawnTimer`
  (returns (RespawnTime :type "Float (double-precision)"))
  (switch `/Game/RTS-Colombia/Blueprints/Enums/RespawnTimerEnum` (`self.TimeSetting`)
    (:`NewEnumerator1`
      (set `self.RespawnTime` 0.0))
    (:`NewEnumerator2`
      (set `self.RespawnTime` (`self.GameSpeed`)))
    (:`NewEnumerator3`
      (set `self.RespawnTime` (`self.UserRespawnTimer`)))
    (:`NewEnumerator4`
      (set `self.RespawnTime` (* (`self.UserRespawnTimer`) (`self.GameSpeed`)))))
  (return (`self.RespawnTime`)))

(fn `SpawnResource`
  (params (Resource :type "/Game/RTS-Colombia/Blueprints/Resources/RTS_ResourcesMaster_Bp Class Reference") (SpawnAmount :type Integer))
  (locals (ResourceLocalRef :type "/Game/RTS-Colombia/Blueprints/Resources/RTS_ResourcesMaster_Bp Class Reference") (SpawnAmountLocal :type Integer))
  (bind (_origin _boxextent) (`self.GetActorBounds` false))
  (bind _x (.x _boxextent))
  (bind _y (.y _boxextent))
  (bind _returnvalue (+ _origin (`KismetMathLibrary.MakeVector` (`KismetMathLibrary.RandomFloatInRange` (- _x (* _x 2.0)) _x) (`KismetMathLibrary.RandomFloatInRange` (- _y (* _y 2.0)) _y) (.z _origin))))
  (set `local.ResourceLocalRef` Resource)
  (set `local.SpawnAmountLocal` SpawnAmount)
  (for _ (range (+ (`local.SpawnAmountLocal`) 1))
    (bind _outhit (`KismetSystemLibrary.BoxTraceSingle` (+ _returnvalue (0.0 0.0 100.0)) (0.0 0.0 0.0) (- _returnvalue (0.0 0.0 100.0)) (struct) "TraceTypeQuery1"))
    (bind (_bblockinghit _binitialoverlap _time _distance _location _impactpoint _normal _impactnormal _physmat _hitactor) (`GameplayStatics.BreakHitResult` _outhit))
    (if (== (`GameplayStatics.GetObjectClass` _hitactor) "/Script/Landscape.Landscape")
      (`|SpawnActorFromClass` (`local.ResourceLocalRef`) (`KismetMathLibrary.Conv_VectorToTransform` _location) "Undefined" "OverrideRootScale" null null))))

(fn `UserConstructionScript`)