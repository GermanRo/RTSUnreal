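; RTS game state that runs the in-game clock and calendar at an adjustable game speed.
; Each Tick advances GameTime through SetGameTime, derives seconds, minutes and hours, rolls days into months and years, and pushes both to the HUD via the cached player controller.
; UpdateGameSpeed scales the default speed by a multiplier and broadcasts it through GameSpeedControl.
; SetGameClock and SetGameCalender are stubs that only return false.
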(event `self.ReceiveBeginPlay`
  (`|ExecutionSequence`
    (:`then_0`
      (`self.ReferenceCasts`))
    (:`then_1`
      ;[1 1 1] ponerGameSpeedDefault
      (set `self.GameTime` (+ (`KismetMathLibrary.Conv_IntToDouble` (`self.Hours`)) (/ (`KismetMathLibrary.Conv_IntToDouble` (`self.Minutes`)) 60.0) (/ (`KismetMathLibrary.Conv_IntToDouble` (`self.Hours`)) 3600.0)))
      (set `self.GameDate` (`|MakeArray` (`self.Day`) (`self.Month`) (`self.Year`))))
    (:`then_2`
      ;[1 1 1] Velocidaddejuego
      (set `self.GameSpeed` (`self.DefaultGameSpeed`)))))

(event `self.ReceiveTick`
  (params (DeltaSeconds :type "Float (single-precision)"))
  (bind (_gametime _daycount) (`/Game/RTS-Colombia/Blueprints/Library/RTS_FuncLib.SetGameTime` DeltaSeconds (`self.GameSpeed`) (`self.GameTime`)))
  (set `self.GameTime` _gametime)
  (set `self.DayCounter` _daycount)
  (`self.Set Clock`)
  (`self.SetCalender`))

(event `/Game/RTS-Colombia/Blueprints/Library/RTS_GameTime_IF.UpdateGameSpeed`
  (params (SpeedMultiplier :type "Float (single-precision)"))
  ;[1 1 1] Actualizar velocidad de juego
  (bind _output_get (set `self.SpeedMultiplier` SpeedMultiplier))
  (bind _output_get_2 (set `self.GameSpeed` (* _output_get (`self.DefaultGameSpeed`))))
  (`self.GameSpeedControl` _output_get_2))

(fn `GetGameSpeed`
  (returns (GameSpeed :type "Float (double-precision)"))
  (return (`self.GameSpeed`)))

(fn `Set Clock`
  (bind (_remainder _returnvalue) (`KismetMathLibrary.FMod` (* (`self.GameTime`) 3600.0) 60.0))
  (bind (_remainder_2 _returnvalue_2) (`KismetMathLibrary.FMod` (`KismetMathLibrary.Conv_IntToDouble` _returnvalue) 60.0))
  (set `self.Seconds` (`KismetMathLibrary.FFloor` _remainder))
  (set `self.Minutes` (`KismetMathLibrary.FFloor` _remainder_2))
  (set `self.Hours` (`KismetMathLibrary.FFloor` (`KismetMathLibrary.FMod` (`KismetMathLibrary.Conv_IntToDouble` _returnvalue_2) 24.0)))
  (bind _output_get (set `self.GameDate` (`|MakeArray` (`self.Seconds`) (`self.Minutes`) (`self.Hours`))))
  (message `/Game/RTS-Colombia/Blueprints/Library/RTS_GameTime_IF.SetGameClock` (`/Game/RTS-Colombia/Blueprints/Player/RTS_PlayerController_BP.HUDGameTimeRef` (`self.ControllerRef`)) _output_get))

(fn `SetCalender`
  (bind _output_get (set `self.Day` (+ (`self.Day`) (`self.DayCounter`))))
  (if (> _output_get (`KismetMathLibrary.DaysInMonth` (`self.Year`) (`self.Month`)))
    (set `self.Day` 1)
    (set `self.Month` (+ (`self.Month`) 1)))
  (if (> (`self.Month`) 12)
    (set `self.Month` 1)
    (set `self.Year` (+ (`self.Year`) 1)))
  (bind _output_get_2 (set `self.GameDate` (`|MakeArray` (`self.Day`) (`self.Month`) (`self.Year`))))
  (message `/Game/RTS-Colombia/Blueprints/Library/RTS_GameTime_IF.SetGameCalender` (`/Game/RTS-Colombia/Blueprints/Player/RTS_PlayerController_BP.HUDGameTimeRef` (`self.ControllerRef`)) _output_get_2))

(fn `SetGameCalender`
  (params (GameDate :type "Array of Integer (by ref)"))
  (returns (Success :type Boolean))
  (return false))

(fn `SetGameClock`
  (params (GameTime :type "Array of Integer (by ref)"))
  (returns (Success :type Boolean))
  (return false))

(fn `UserConstructionScript`)