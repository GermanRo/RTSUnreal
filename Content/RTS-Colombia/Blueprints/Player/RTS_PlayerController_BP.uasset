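; RTS player controller that handles camera, unit selection and orders, and building placement.
; On BeginPlay it caches camera pawn, game state and marquee HUD, then spawns the construction preview, construction master and main UI.
; Camera supports axis movement, edge scrolling, gated mouse panning and zoom.
; Building mode switches clicks from marquee selection and AI move orders with decals to placing or cancelling a rotatable preview; V spawns a unit at the cursor.
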(event `self.ReceiveBeginPlay`
  (`|ExecutionSequence`
    (:`then_0`
      (`self.ReferenceCast`) ; Debe ser primero
    )
    (:`then_1`
      (bind _returnvalue (`|SpawnActorFromClass` "/Game/RTS-Colombia/Blueprints/Buildings/RTS_PreviewBuilding.RTS_PreviewBuilding_C" (`self.Empty trasnform`) "AlwaysSpawn" "OverrideRootScale" null self null))
      (set `self.ConstructionPreviewRef` _returnvalue)
      (bind _returnvalue_2 (`|SpawnActorFromClass` "/Game/RTS-Colombia/Blueprints/Buildings/RTS_ConstructionMasterBP.RTS_ConstructionMasterBP_C" (`self.Empty trasnform`) "Undefined" "OverrideRootScale" null self null))
      (set `self.ConstructionMaster Ref` _returnvalue_2))
    (:`then_2`
      (`self.SpawnWidget`)
      (`UserWidget.AddToViewport` (`self.HUDMainGame`) 1)
      (`self.SetHUDVisibility` "Visible"))
    (:`then_3`
      (`WidgetBlueprintLibrary.SetInputMode_GameAndUIEx` self null "DoNotLock" false))))

(event `self.ReceiveTick`
  (params (DeltaSeconds :type "Float (single-precision)"))
  (set `self.DeltaTime` DeltaSeconds)
  (if (`self.IsHoldingInput`)
    (`self.UpdateSelection`)
    (elif (and (`self.IsBuildingModeActive`) (!= (`self.ConstructionPreviewRef`) null))
      (`/Game/RTS-Colombia/Blueprints/Buildings/RTS_PreviewBuilding.GetCursorPOsition` (`self.ConstructionPreviewRef`) (`/Game/RTS-Colombia/Blueprints/Library/RTS_FuncLib.SetCursorWorldPosition` self 10000.0)))))

(event `InputAction|RotatePreviewLeft`
  (params (Key :type "Key Structure"))
  (bind _constructionpreviewref (`self.ConstructionPreviewRef`))
  (bind (_returnvalue_roll _returnvalue_pitch _returnvalue_yaw) (`KismetMathLibrary.BreakRotator` (`self.K2_GetActorRotation` _constructionpreviewref)))
  ;[1 1 1] Girar Construcciones
  (:`Pressed`
    (if (and (`self.IsBuildingModeActive`) (!= _constructionpreviewref null))
      (`self.K2_SetActorRotation` _constructionpreviewref (`KismetMathLibrary.MakeRotator` _returnvalue_roll _returnvalue_pitch (+ _returnvalue_yaw (`self.ConstructionRotationRate`))) false))))

(event `InputAction|ZoomReset`
  (params (Key :type "Key Structure"))
  ;[1 1 1] Resetear al zoom
  (:`Pressed`
    (set `SpringArmComponent.TargetArmLength` 1500.0 (`/Game/RTS-Colombia/Blueprints/Player/RTS_CamaraPawn_BP.SpringArm` (`self.CameraPawnRef`)))))

(event `InputAction|SpeedModifier`
  (params (Key :type "Key Structure"))
  ;[1 1 1] Movimeinto de camara
  ;;[1 1 1] Set VELOCIDAD DE MOVIMENTO CAMARA
  (:`Pressed`
    (set `self.MovementSpeedModifier` 2.0))
  (:`Released`
    (set `self.MovementSpeedModifier` 1.0)))

(event `InputAction|ZoomIn`
  (params (Key :type "Key Structure"))
  (bind _springarm (`/Game/RTS-Colombia/Blueprints/Player/RTS_CamaraPawn_BP.SpringArm` (`self.CameraPawnRef`)))
  ;[1 1 1] Zoom in y out
  (:`Pressed`
    (set `SpringArmComponent.TargetArmLength` (`KismetMathLibrary.FClamp` (- (`SpringArmComponent.TargetArmLength` _springarm) (`self.ZoomSpeed`)) (`self.MinZoomLimit`) (`self.MaxZoomLimit`)) _springarm)))

(event `InputAxis|MoveForward`
  (params (AxisValue :type "Float (single-precision)"))
  ;[1 1 1] Movimeinto de camara
  ;;[1 1 1] Mover camara hacia arriba y bajo
  (if (not (`self.DisableCamMovement`))
    ;;[1 1 1] Mover camara hacia izq y der
    (`self.FuncionesDeMovimientodeCamara` AxisValue (stale `InputAxis|MoveRight` AxisValue) :!label _label)))

(event `InputAxis|MoveRight`
  (params (AxisValue :type "Float (single-precision)"))
  ;[1 1 1] Movimeinto de camara
  ;;[1 1 1] Mover camara hacia izq y der
  (if (not (`self.DisableCamMovement`))
    (goto _label :!via `Movimiento Der`)))

(event `InputAction|RotatePreviewRight`
  (params (Key :type "Key Structure"))
  (bind _constructionpreviewref (`self.ConstructionPreviewRef`))
  (bind (_returnvalue_roll _returnvalue_pitch _returnvalue_yaw) (`KismetMathLibrary.BreakRotator` (`self.K2_GetActorRotation` _constructionpreviewref)))
  ;[1 1 1] Girar Construcciones
  (:`Pressed`
    (if (and (`self.IsBuildingModeActive`) (!= _constructionpreviewref null))
      (`self.K2_SetActorRotation` _constructionpreviewref (`KismetMathLibrary.MakeRotator` _returnvalue_roll _returnvalue_pitch (- _returnvalue_yaw (`self.ConstructionRotationRate`))) false))))

(event `InputAction|ZoomOut`
  (params (Key :type "Key Structure"))
  (bind _springarm (`/Game/RTS-Colombia/Blueprints/Player/RTS_CamaraPawn_BP.SpringArm` (`self.CameraPawnRef`)))
  ;[1 1 1] Zoom in y out
  (:`Pressed`
    (set `SpringArmComponent.TargetArmLength` (`KismetMathLibrary.FClamp` (+ (`self.ZoomSpeed`) (`SpringArmComponent.TargetArmLength` _springarm)) (`self.MinZoomLimit`) (`self.MaxZoomLimit`)) _springarm)))

(event `InputAxisKey|MouseX`
  (params (AxisValue :type "Float (single-precision)"))
  ;[1 1 1] Movimeinto de camara
  ;;[1 1 1] EdgeScrollMovement
  (if (not (`self.DisableCamMovement`))
    (bind (_deltaspeedx _deltaspeedy) (`self.EdgeScroll` :!label _label_2))
    (`self.K2_AddActorLocalOffset` (`self.CameraPawnRef`) (`KismetMathLibrary.MakeVector` _deltaspeedx _deltaspeedy) true false)))

(event `InputAxisKey|MouseY`
  (params (AxisValue :type "Float (single-precision)"))
  ;[1 1 1] Movimeinto de camara
  ;;[1 1 1] EdgeScrollMovement
  (if (not (`self.DisableCamMovement`))
    (goto _label_2 :!via `MouseY`)))

(event `InputAction|PanReset`
  (params (Key :type "Key Structure"))
  (bind _camerapawnref (`self.CameraPawnRef`))
  ;[1 1 1] ResetPan
  (:`Pressed`
    (`self.K2_SetActorRotation` _camerapawnref (`KismetMathLibrary.MakeRotator` (.roll (`self.K2_GetActorRotation` _camerapawnref)) 0.0 (.yaw (`self.K2_GetActorRotation` _camerapawnref))) false)))

(event `InputAction|Pan`
  (params (Key :type "Key Structure"))
  (bind _camerapawnref (`self.CameraPawnRef`))
  ;[1 1 1] PANX
  (:`Pressed`
    (set `self.DisableCamMovement` true)
    (goto _label_3 :!via `Open`))
  (:`Released`
    (set `self.DisableCamMovement` false)
    (goto _label_3 :!via `Close`)))

(event `Key|V`
  (params (Key :type "Key Structure"))
  (bind (_relativecursorlocationingame_x _relativecursorlocationingame_y) (`KismetMathLibrary.BreakVector` (`/Game/RTS-Colombia/Blueprints/Library/RTS_FuncLib.SetCursorWorldPosition` self 10000.0)))
  (:`Pressed`
    (bind _returnvalue (`|SpawnActorFromClass` "/Game/RTS-Colombia/Unidades/RTS_UnidadMaster.RTS_UnidadMaster_C" (`KismetMathLibrary.MakeTransform` (`KismetMathLibrary.MakeVector` _relativecursorlocationingame_x _relativecursorlocationingame_y -347.0)) "Undefined" "OverrideRootScale" null null))
    (set `self.SpawnedUnit` _returnvalue)))

(event `InputAxisKey|MouseX`
  (params (AxisValue :type "Float (single-precision)"))
  (bind _camerapawnref (`self.CameraPawnRef`))
  ;[1 1 1] PANX
  (`/Engine/EditorBlueprintResources/StandardMacros.Gate` true :!label _label_3
    (:`Exit`
      (`self.K2_SetActorRotation` _camerapawnref (`KismetMathLibrary.MakeRotator` (.roll (`self.K2_GetActorRotation` _camerapawnref)) (.pitch (`self.K2_GetActorRotation` _camerapawnref)) (+ (.yaw (`self.K2_GetActorRotation` _camerapawnref)) (* AxisValue (`self.Pan Speed`)))) false))))

(event `InputAction|PrimaryAction`
  (params (Key :type "Key Structure"))
  (:`Pressed`
    (if (`self.IsBuildingModeActive`)
      (if (not (`/Game/RTS-Colombia/Blueprints/Buildings/RTS_PreviewBuilding.CheckOverlap` (`self.ConstructionPreviewRef`)))
        (bind _constructionstruct (`/Game/RTS-Colombia/Blueprints/Buildings/RTS_PreviewBuilding.SetConstructionStructure` (`self.ConstructionPreviewRef`)))
        (`/Game/RTS-Colombia/Blueprints/Buildings/RTS_ConstructionMasterBP.StartConstruction` (`self.ConstructionMaster Ref`) _constructionstruct)
        (`/Game/RTS-Colombia/Blueprints/Buildings/RTS_PreviewBuilding.DestroyPreview` (`self.ConstructionPreviewRef`)))
      (else
        (message `/Game/RTS-Colombia/Blueprints/Library/RTS_MarqueeSelection_IF.OnInputStart` (`self.MarqueeRef`))
        (set `self.HoldingTime` 0.0)
        (set `self.IsHoldingInput` true))))
  (:`Released`
    (if (not (`self.IsBuildingModeActive`))
      (message `/Game/RTS-Colombia/Blueprints/Library/RTS_MarqueeSelection_IF.OnInputRelease` (`self.MarqueeRef`) (`self.HoldingTime`))
      (set `self.IsHoldingInput` false))))

(event `InputAction|Pan`
  (params (Key :type "Key Structure"))
  (bind _camerapawnref (`self.CameraPawnRef`))
  ;[1 1 1] PANY
  (:`Pressed`
    (set `self.DisableCamMovement` true)
    (goto _label_4 :!via `Open`))
  (:`Released`
    (set `self.DisableCamMovement` false)
    (goto _label_4 :!via `Close`)))

(event `InputAxisKey|MouseY`
  (params (AxisValue :type "Float (single-precision)"))
  (bind _camerapawnref (`self.CameraPawnRef`))
  ;[1 1 1] PANY
  (`/Engine/EditorBlueprintResources/StandardMacros.Gate` true :!label _label_4
    (:`Exit`
      (`self.K2_SetActorRotation` _camerapawnref (`KismetMathLibrary.MakeRotator` (.roll (`self.K2_GetActorRotation` _camerapawnref)) (`KismetMathLibrary.FClamp` (+ (.pitch (`self.K2_GetActorRotation` _camerapawnref)) (* AxisValue (`self.Pan Speed`))) -25.0 45.0) (.yaw (`self.K2_GetActorRotation` _camerapawnref))) false))))

(event `UpdateSelection`
  (if (`self.IsHoldingInput`)
    (set `self.HoldingTime` (+ (`self.HoldingTime`) (`self.DeltaTime`)))
    (message `/Game/RTS-Colombia/Blueprints/Library/RTS_MarqueeSelection_IF.OnInputHold` (`self.MarqueeRef`))))

(event `InputAction|SecondaryAction`
  (params (Key :type "Key Structure"))
  (bind (_hitresult _returnvalue) (`self.GetHitResultUnderCursorByChannel` "TraceTypeQuery1" false))
  (bind _previouslocationdecal (`self.PreviousLocationDecal`))
  (bind _previouslocationdecal_2 (`self.PreviousLocationDecal`))
  ;[1 1 1] Info NPC
  (:`Pressed`
    (if (`self.IsBuildingModeActive`)
      (`/Game/RTS-Colombia/Blueprints/Buildings/RTS_PreviewBuilding.DestroyPreview` (`self.ConstructionPreviewRef`))
      (elif (`self.IsUnitSelected`)
        (if _returnvalue
          (set `self.TargetLocation` (`.Location` (`GameplayStatics.BreakHitResult` _hitresult)))
          (`|ExecutionSequence`
            (:`then_0`
              ;[1 1 1] Verificar punto de movimiento (azul)
              (`/Engine/EditorBlueprintResources/StandardMacros.IsValid` _previouslocationdecal_2
                (:`Is Valid`
                  (`ActorComponent.K2_DestroyComponent` _previouslocationdecal_2)
                  (bind _returnvalue_2 (`AIBlueprintHelperLibrary.GetAIController` (stale _array_element)))
                  (`self.StopMovement` _returnvalue_2))
                (:`Is Not Valid`
                  _))
              (bind _returnvalue_3 (`GameplayStatics.SpawnDecalAtLocation` "/Game/RTS-Colombia/Materiales/Etiquetas_SeleccionMovimiento/Etiqueta_MovmentLocation.Etiqueta_MovmentLocation" (32.0 64.0 64.0) (`self.TargetLocation`)))
              (set `self.PreviousLocationDecal` _returnvalue_3))
            (:`then_1`
              (for _array_element (`self.SelectedUnits`)
                (`self.StopMovement` _returnvalue_2)
                (`AITask_MoveTo.AIMoveTo` _returnvalue_2 (`self.TargetLocation`) null -1.0 "Disable" "Enable" true false
                  (:`OnMoveFinished`
                    (`/Engine/EditorBlueprintResources/StandardMacros.IsValid` _previouslocationdecal
                      (:`Is Valid`
                        (`ActorComponent.K2_DestroyComponent` _previouslocationdecal)))))))))
        (else
          (`self.GetUnitHUD`))))))

(fn `Despausar`
  (bind _returnvalue (`GameplayStatics.GetPlayerController` 0))
  (`GameplayStatics.SetGamePaused` false)
  (`WidgetLayoutLibrary.RemoveAllWidgets`)
  (`WidgetBlueprintLibrary.SetInputMode_GameOnly` _returnvalue)
  (set `PlayerController.bShowMouseCursor` false _returnvalue))

(fn `GetUnitHUD`
  (bind (_bblockinghit _binitialoverlap _time _distance _location _impactpoint _normal _impactnormal _physmat _hitactor) (`GameplayStatics.BreakHitResult` (`self.GetHitResultUnderCursorForObjects` (`self.SelectableObjectsEnum`))))
  (if (!= _hitactor null)
    (`self.DisplayHUD` _hitactor)))

(fn `PauseGame`
  (`GameplayStatics.SetGamePaused` true)
  (`/Engine/EditorBlueprintResources/StandardMacros.IsValid` (`self.VariablePausa`)
    (:`Is Valid`
      _)
    (:`Is Not Valid`
      (bind _returnvalue (`|CreateWidget` "/Game/TopDownBP/Maps/Pausa.Pausa_C" (`GameplayStatics.GetPlayerController` 0)))
      (set `self.VariablePausa` _returnvalue)))
  (`UserWidget.AddToViewport` (`self.VariablePausa`) 0)
  (`WidgetBlueprintLibrary.SetInputMode_UIOnlyEx` (`GameplayStatics.GetPlayerController` 0) (`self.VariablePausa`))
  (set `PlayerController.bShowMouseCursor` true (`GameplayStatics.GetPlayerController` 0)))

(fn `SetBuildingModeActive`
  (params (IsActive :type Boolean))
  (set `self.IsBuildingModeActive` IsActive)
  (return))

(fn `SetHUDVisibility`
  (params (GameTimeHUD :type "ESlateVisibility Enum" :default "Visible"))
  (`Widget.SetVisibility` (`self.HUDMainGame`) GameTimeHUD))

(fn `SetSelectedUnits`
  (params (SelectedUnits :type "Array of /Game/RTS-Colombia/Unidades/RTS_UnidadMaster Object Reference"))
  (set `self.SelectedUnits` SelectedUnits)
  (if (>= (`KismetArrayLibrary.Array_LastIndex` (`self.SelectedUnits`)) 0)
    (set `self.IsUnitSelected` true)))

(fn `UserConstructionScript`)