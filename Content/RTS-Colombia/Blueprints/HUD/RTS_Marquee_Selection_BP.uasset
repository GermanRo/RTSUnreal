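; RTS HUD that draws a drag-selection rectangle and gathers units under it.
; Input events record mouse corners, clear the previous selection on press and pass SelectedUnits to the player controller on release.
; While dragging, DrawHUD queries the rectangle separately for Machete, FusileroCriollo and Harvester units, adding them uniquely without removing any that leave.
; Deselection resets decals and flags, but the code setting them on selection is disconnected.
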(event `self.ReceiveBeginPlay`
  (set `self.ControllerRef` (cast `/Game/RTS-Colombia/Blueprints/Player/RTS_PlayerController_BP` (`GameplayStatics.GetPlayerController` 0) :!pure true)))

(event `/Game/RTS-Colombia/Blueprints/Library/RTS_MarqueeSelection_IF.OnInputHold`
  (bind (_locationx _locationy) (`PlayerController.GetMousePosition` (`self.ControllerRef`)))
  (set `self.HoldingLocation` (`KismetMathLibrary.MakeVector2D` _locationx _locationy)))

(event `/Game/RTS-Colombia/Blueprints/Library/RTS_MarqueeSelection_IF.OnInputStart`
  (bind (_locationx _locationy) (`PlayerController.GetMousePosition` (`self.ControllerRef`)))
  ;[1 1 1] Selección de area (verifica si la matriz de selección está vacía o no)
  (if (>= (`KismetArrayLibrary.Array_LastIndex` (`self.SelectedUnits`)) 0)
    (for _array_element (`self.SelectedUnits`)
      (`/Game/RTS-Colombia/Unidades/RTS_UnidadMaster.SetDeselectedDecal` _array_element)
      (set `/Game/RTS-Colombia/Unidades/RTS_UnidadMaster.IsSelected` false _array_element)
      (set `/Game/RTS-Colombia/Blueprints/Player/RTS_PlayerController_BP.IsUnitSelected` false (`self.ControllerRef`)))
    (`KismetArrayLibrary.Array_Clear` (`self.SelectedUnits`)))
  (bind _output_get (set `self.ClickedLocation` (`KismetMathLibrary.MakeVector2D` _locationx _locationy)))
  (set `self.HoldingLocation` _output_get)
  (set `self.IsDrawing` true))

(event `/Game/RTS-Colombia/Blueprints/Library/RTS_MarqueeSelection_IF.OnInputRelease`
  (params (HoldTime :type "Float (single-precision)"))
  (set `self.IsDrawing` false)
  (`/Game/RTS-Colombia/Blueprints/Player/RTS_PlayerController_BP.SetSelectedUnits` (`self.ControllerRef`) (`self.SelectedUnits`)))

(event `self.ReceiveDrawHUD`
  (params (SizeX :type Integer) (SizeY :type Integer))
  (if (`self.IsDrawing`)
    (`|ExecutionSequence`
      (:`then_0`
        (`self.DrawMarquee`)
        (bind _output_get (set `self.UnitsInSelectionArea` (`self.GetActorsInSelectionRectangle` "/Game/RTS-Colombia/Unidades/RTS_MacheteUnit.RTS_MacheteUnit_C" (`self.ClickedLocation`) (`self.HoldingLocation`) false)))
        (for _array_element _output_get
          (if (`KismetMathLibrary.ClassIsChildOf` (`GameplayStatics.GetObjectClass` _array_element) "/Game/RTS-Colombia/Unidades/RTS_UnidadMaster.RTS_UnidadMaster_C")
            (bind _asrts_unidad_master (cast `/Game/RTS-Colombia/Unidades/RTS_UnidadMaster` _array_element))
            (set `self.SelectedUnit` _asrts_unidad_master)
            (`|ExecutionSequence`
              (:`then_0`
                (`KismetArrayLibrary.Array_AddUnique` (`self.SelectedUnits`) (`self.SelectedUnit`)))
              (:`then_1`
                (for _array_element_2 (`self.SelectedUnits`)
                  _))))))
      (:`then_1`
        (`self.DrawMarquee`)
        (bind _output_get_2 (set `self.UnitsInSelectionArea` (`self.GetActorsInSelectionRectangle` "/Game/RTS-Colombia/Unidades/RTS_FusileroCriolloUnit.RTS_FusileroCriolloUnit_C" (`self.ClickedLocation`) (`self.HoldingLocation`) false)))
        (for _array_element_3 _output_get_2
          (if (`KismetMathLibrary.ClassIsChildOf` (`GameplayStatics.GetObjectClass` _array_element_3) "/Game/RTS-Colombia/Unidades/RTS_UnidadMaster.RTS_UnidadMaster_C")
            (bind _asrts_unidad_master_2 (cast `/Game/RTS-Colombia/Unidades/RTS_UnidadMaster` _array_element_3))
            (set `self.SelectedUnit` _asrts_unidad_master_2)
            (`|ExecutionSequence`
              (:`then_0`
                (`KismetArrayLibrary.Array_AddUnique` (`self.SelectedUnits`) (`self.SelectedUnit`)))
              (:`then_1`
                (for _array_element_4 (`self.SelectedUnits`)
                  _))))))
      (:`then_2`
        (`self.DrawMarquee`)
        (bind _output_get_3 (set `self.UnitsInSelectionArea` (`self.GetActorsInSelectionRectangle` "/Game/RTS-Colombia/Unidades/RTS_HarvesterUnit.RTS_HarvesterUnit_C" (`self.ClickedLocation`) (`self.HoldingLocation`) false)))
        (for _array_element_5 _output_get_3
          (if (`KismetMathLibrary.ClassIsChildOf` (`GameplayStatics.GetObjectClass` _array_element_5) "/Game/RTS-Colombia/Unidades/RTS_UnidadMaster.RTS_UnidadMaster_C")
            (bind _asrts_unidad_master_3 (cast `/Game/RTS-Colombia/Unidades/RTS_UnidadMaster` _array_element_5))
            (set `self.SelectedUnit` _asrts_unidad_master_3)
            (`|ExecutionSequence`
              (:`then_0`
                (`KismetArrayLibrary.Array_AddUnique` (`self.SelectedUnits`) (`self.SelectedUnit`)))
              (:`then_1`
                (for _array_element_6 (`self.SelectedUnits`)
                  _)))))))))

(event `DrawMarquee`
  (bind _clickedlocation (`self.ClickedLocation`))
  (bind (_x _y) (`KismetMathLibrary.BreakVector2D` (`self.HoldingLocation`)))
  (bind (_x_2 _y_2) (`KismetMathLibrary.BreakVector2D` _clickedlocation))
  (bind (_x_3 _y_3) (`KismetMathLibrary.BreakVector2D` (`self.ClickedLocation`)))
  (bind (_x_4 _y_4) (`KismetMathLibrary.BreakVector2D` (- (`self.HoldingLocation`) _clickedlocation)))
  ;[1 1 1] Dibujar cuadro de seleccion
  (`self.DrawRect` (struct :`R` 0.786458 :`G` 0.143365 :`B` 0.143365) _x_3 _y_3)
  (`self.DrawRect` (struct :`R` 0.225145 :`G` 0.263783 :`B` 0.9375) _x _y)
  (`self.DrawRect` (struct :`R` 0.1199 :`G` 0.858016 :`B` 0.885417 :`A` 0.504) _x_2 _y_2 _x_4 _y_4))

(fn `UserConstructionScript`)