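; Ghost preview actor for RTS building placement, showing the chosen building's mesh and toggling building mode on the player controller.
; While previewing, a gated Tick moves it to the grid-snapped cursor position and swaps its material when it overlaps any actor.
; ConstructBuilding briefly spawns the building class to read its details, restarts the preview with them, then destroys that instance.
; SetConstructionStructure packages the details and transform into a construction struct.
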(event `Spawn Preview`
  (params (BuildingClass :type "/Game/RTS-Colombia/Blueprints/Buildings/RTS_BuildingMaster_BP Class Reference") (DisplayMesh :type "StaticMesh Object Reference") (ConstructionTime :type "Float (double-precision)") (BuildingName :type "/Game/RTS-Colombia/Blueprints/Enums/BuildingNameEnum Enum" :default "NewEnumerator0") (WoodCost :type "Float (double-precision)") (RockCost :type "Float (double-precision)"))
  (if (`self.IsPreviewing`)
    (`self.DestroyPreview`))
  (`self.SetBuildingDetails` BuildingClass DisplayMesh ConstructionTime BuildingName WoodCost RockCost)
  (bind _output_get (set `self.IsPreviewing` true))
  (`/Game/RTS-Colombia/Blueprints/Player/RTS_PlayerController_BP.SetBuildingModeActive` (`self.PlayerControllerRef`) _output_get)
  (`StaticMeshComponent.SetStaticMesh` (`self.PreviewBuildingMesh`) (`self.DisplayMesh`))
  (`self.OpenGate`))

(event `DestroyPreview`
  (`self.CloseGate`)
  (set `self.Building Class` null)
  (set `self.DisplayMesh` null)
  (bind _output_get (set `self.IsPreviewing` false))
  (`/Game/RTS-Colombia/Blueprints/Player/RTS_PlayerController_BP.SetBuildingModeActive` (`self.PlayerControllerRef`) _output_get)
  (`StaticMeshComponent.SetStaticMesh` (`self.PreviewBuildingMesh`) (`self.DisplayMesh`))
  (`self.K2_SetActorLocation` (0.0 0.0 0.0)))

(event `/Game/RTS-Colombia/Blueprints/Library/RTS_CONTRUCTIONIF.ConstructBuilding`
  (params (BuildingMasterClass :type "/Game/RTS-Colombia/Blueprints/Buildings/RTS_BuildingMaster_BP Class Reference"))
  (bind _returnvalue (`|SpawnActorFromClass` BuildingMasterClass (`self.EmptyTransform`) "AlwaysSpawn" "OverrideRootScale" null (`self.PlayerControllerRef`) null "NewEnumerator0" null))
  (`|ExecutionSequence`
    (:`then_0`
      (bind _asrts_building_master_bp (castclass `/Game/RTS-Colombia/Blueprints/Buildings/RTS_BuildingMaster_BP` BuildingMasterClass))
      (`self.DestroyPreview`)
      (`self.Spawn Preview` _asrts_building_master_bp (`/Game/RTS-Colombia/Blueprints/Buildings/RTS_BuildingMaster_BP.DisplayMesh` _returnvalue) (`/Game/RTS-Colombia/Blueprints/Buildings/RTS_BuildingMaster_BP.ConstructionTime` _returnvalue) (`/Game/RTS-Colombia/Blueprints/Buildings/RTS_BuildingMaster_BP.BuildingName` _returnvalue) (`/Game/RTS-Colombia/Blueprints/Buildings/RTS_BuildingMaster_BP.WoodCost` _returnvalue) (`/Game/RTS-Colombia/Blueprints/Buildings/RTS_BuildingMaster_BP.RockCost` _returnvalue)))
    (:`then_1`
      (`self.K2_DestroyActor` _returnvalue))))

(event `self.ReceiveTick`
  (params (DeltaSeconds :type "Float (single-precision)"))
  (bind _previewbuildingmesh (`self.PreviewBuildingMesh`))
  (`/Engine/EditorBlueprintResources/StandardMacros.Gate` true :!label _label
    (:`Exit`
      (`self.K2_SetActorLocation` self (`self.GridSnaps`) false false)
      (if (`self.CheckOverlap`)
        (`PrimitiveComponent.SetMaterial` _previewbuildingmesh 0 "/Game/RTS-Colombia/Materiales/Etiquetas_SeleccionMovimiento/Construccion/PreviewBAD_Inst.PreviewBAD_Inst")
        (else
          (`PrimitiveComponent.SetMaterial` _previewbuildingmesh 0 "/Game/RTS-Colombia/Materiales/Etiquetas_SeleccionMovimiento/Construccion/Preview_M_Inst.Preview_M_Inst"))))))

(event `OpenGate`
  (goto _label :!via `Open`))

(event `CloseGate`
  (goto _label :!via `Close`))

(fn `CheckOverlap`
  (returns (IsOverlapping :type Boolean))
  (return (>= (`KismetArrayLibrary.Array_LastIndex` (`self.GetOverlappingActors` null)) 0)))

(fn `GetCursorPOsition`
  (params (CursorLocationIn :type "Vector Structure"))
  (set `self.CursorWorldPosition` CursorLocationIn)
  (return))

(fn `GridSnaps`
  (returns (SnapPosition :type "Vector Structure"))
  (bind (_cursorworldposition_x _cursorworldposition_y _cursorworldposition_z) (`KismetMathLibrary.BreakVector` (`self.CursorWorldPosition`)))
  (bind _snapvalue (`self.SnapValue`))
  (bind _snapvalue_2 (`self.SnapValue`))
  (return (`KismetMathLibrary.MakeVector` (`KismetMathLibrary.Conv_IntToDouble` (* (/ (`KismetMathLibrary.FFloor` (+ _cursorworldposition_x 50.0)) _snapvalue_2) _snapvalue_2)) (`KismetMathLibrary.Conv_IntToDouble` (* (/ (`KismetMathLibrary.FFloor` (+ _cursorworldposition_y 50.0)) _snapvalue) _snapvalue)) _cursorworldposition_z)))

(fn `SetBuildingDetails`
  (params (`Building Class` :type "/Game/RTS-Colombia/Blueprints/Buildings/RTS_BuildingMaster_BP Class Reference") (DisplayMesh :type "StaticMesh Object Reference") (ConstructionHours :type "Float (double-precision)") (BuildignName :type "/Game/RTS-Colombia/Blueprints/Enums/BuildingNameEnum Enum" :default "NewEnumerator0") (WoodCost :type "Float (double-precision)") (RockCost :type "Float (double-precision)"))
  (set `self.Building Class` `Building Class`)
  (set `self.DisplayMesh` DisplayMesh)
  (set `self.ConstructionHours` ConstructionHours)
  (set `self.BuildingName` BuildignName)
  (set `self.WoodCost` WoodCost)
  (set `self.RockCost` RockCost))

(fn `SetConstructionStructure`
  (returns (ConstructionStruct :type "/Game/RTS-Colombia/Blueprints/Structures/RTS_ContructionStruct Structure"))
  (set `self.ConstructionStruct` (make `/Game/RTS-Colombia/Blueprints/Structures/RTS_ContructionStruct` false (`self.Building Class`) (`KismetMathLibrary.MakeTransform` (`self.K2_GetActorLocation`) (`self.K2_GetActorRotation`)) (`self.DisplayMesh`) (`self.BuildingName`) (`self.ConstructionHours`)))
  (return (`self.ConstructionStruct`)))

(fn `UserConstructionScript`)