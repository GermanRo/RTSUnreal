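; Master Blueprint for RTS buildings, handling construction, unit occupancy, health and HUD.
; The construction script applies the mesh, entry box and preview material; harvesters overlapping the box report arrival if targeting this building.
; While occupied and unbuilt, Tick advances work by game speed and occupant count, then on completion releases occupants and updates the player controller.
; Otherwise, the status bar turns toward the camera; controller events open the info HUD.
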(event `self.ReceiveBeginPlay`
  ;[1 1 1] GENERAL to ALL BUILDINGS
  (`|ExecutionSequence`
    (:`then_0`
      (`self.ReferencesCast`))
    (:`then_1`
      (add `/Game/RTS-Colombia/Blueprints/GameSettings/RTS_GameState_BP.GameSpeedControl` (`self.GameStateRef`) (`|CreateDelegate` :!event `GetGameSpeed`))
      (bind _gamespeed (`/Game/RTS-Colombia/Blueprints/GameSettings/RTS_GameState_BP.GetGameSpeed` (`self.GameStateRef`)))
      (set `self.GameSpeed` _gamespeed))
    (:`then_2`
      (if (`self.IsBuilt`)
        (`self.UpdateBuildingHealth`)
        (`self.SetArmorBarHidden`)))
    (:`then_3`
      (add `/Game/RTS-Colombia/Blueprints/Player/RTS_PlayerController_BP.DisplayHUD` (`self.PlayerControllerRef`) (`|CreateDelegate` :!event `DisplayBuildingHUD`)))))

(event `OnSpawn`
  ;[1 1 1] GENERAL to ALL BUILDINGS
  (set `self.IsUnderConstruction` true))

(event `GetGameSpeed`
  (params (GameSpeed :type "Float (double-precision)"))
  ;[1 1 1] GENERAL to ALL BUILDINGS
  (set `self.GameSpeed` GameSpeed))

(event `self.ReceiveTick`
  (params (DeltaSeconds :type "Float (single-precision)"))
  (bind _playercontrollerref (`self.PlayerControllerRef`))
  ;[1 1 1] GENERAL to ALL BUILDINGS
  (set `self.DeltaTime` DeltaSeconds)
  (if (and (`self.IsUnderConstruction`) (not (`self.IsBuilt`)) (>= (`KismetArrayLibrary.Array_LastIndex` (`self.Occupants`)) 0))
    (`self.ConstructBuilding`)
    (if (>= (`self.TimeWorked`) (`self.ConstructionTime`))
      (set `self.IsBuilt` true)
      (set `self.IsUnderConstruction` false)
      (`self.ReleaseAllOccupants`)
      (`self.ClearOccupantsList`)
      (`PrimitiveComponent.SetMaterial` (`self.BuildingMesh`) 0 null)
      (`self.SetStatusBarVIsible`)
      (`self.UpdateBuildingHealth`)
      (`self.SetStatusBarVIsible`)
      (`/Game/RTS-Colombia/Blueprints/Player/RTS_PlayerController_BP.UpdateBuildignList` _playercontrollerref)
      (`/Game/RTS-Colombia/Blueprints/Player/RTS_PlayerController_BP.SetMaxResources` _playercontrollerref))
    (else
      (`self.OrientToCamera`))))

(event `DisplayBuildingHUD`
  (params (Actor :type "Actor Object Reference") (Bypass :type Boolean))
  (bind _playercontrollerref (`self.PlayerControllerRef`))
  ;[1 1 1] GENERAL to ALL BUILDINGS
  (if (== Actor self)
    (`UserWidget.AddToViewport` (`self.BuildingHUD`) 1)
    (`WidgetBlueprintLibrary.SetInputMode_UIOnlyEx` _playercontrollerref null)
    (`Widget.SetIsEnabled` (`/Game/RTS-Colombia/Blueprints/Player/RTS_PlayerController_BP.HUDMainGame` _playercontrollerref) true)))

(event `self.EntryPoint.OnComponentBeginOverlap`
  (params (OverlappedComponent :type "PrimitiveComponent Object Reference") (OtherActor :type "Actor Object Reference") (OtherComp :type "PrimitiveComponent Object Reference") (OtherBodyIndex :type Integer) (bFromSweep :type Boolean) (SweepResult :type "HitResult Structure (by ref)"))
  ;[1 1 1] GENERAL to ALL BUILDINGS
  (if (`KismetMathLibrary.ClassIsChildOf` (`GameplayStatics.GetObjectClass` OtherActor) "/Game/RTS-Colombia/Unidades/RTS_HarvesterUnit.RTS_HarvesterUnit_C")
    (bind _asrts_unidad_master (cast `/Game/RTS-Colombia/Unidades/RTS_UnidadMaster` OtherActor))
    (set `self.SelectedUnit` _asrts_unidad_master)
    (if (== (`/Game/RTS-Colombia/Unidades/RTS_UnidadMaster.TargetBuilding` (`self.SelectedUnit`)) self)
      (`/Game/RTS-Colombia/Unidades/RTS_UnidadMaster.ArriveBuilding` (`self.SelectedUnit`)))))

(event `RecruitmentTrigger`)

(fn `ClearOccupantsList`
  (`KismetArrayLibrary.Array_Clear` (`self.Occupants`))
  (message `/Game/RTS-Colombia/Blueprints/Library/RTS_OccupantiNFO.SetOccupantName` (`self.BuildingHUD`) (`self.Occupants`))
  (`/Game/RTS-Colombia/Blueprints/Widgets/BuildingInfo_HUD.UpdateOccupantList` (`self.BuildingHUD`))
  (return))

(fn `ConstructBuilding`
  (bind _output_get (set `self.GameClock` (`/Game/RTS-Colombia/Blueprints/Library/RTS_FuncLib.SetGameTime` (`self.DeltaTime`) (/ (`self.GameSpeed`) (`KismetMathLibrary.Conv_IntToDouble` (`KismetArrayLibrary.Array_Length` (`self.Occupants`)))) (`self.GameClock`))))
  (set `self.TimeWorked` (* _output_get (`self.ConstructionModifer`) 60.0))
  (return))

(fn `GetUnit`
  (params (TargetUnit :type "/Game/RTS-Colombia/Unidades/RTS_UnidadMaster Object Reference"))
  (`KismetArrayLibrary.Array_AddUnique` (`self.Occupants`) TargetUnit)
  (message `/Game/RTS-Colombia/Blueprints/Library/RTS_OccupantiNFO.SetOccupantName` (`self.BuildingHUD`) (`self.Occupants`))
  (`/Game/RTS-Colombia/Blueprints/Widgets/BuildingInfo_HUD.UpdateOccupantList` (`self.BuildingHUD`))
  (return))

(fn `OrientToCamera`
  (bind (_relativerotation_roll _relativerotation_pitch _relativerotation_yaw) (`KismetMathLibrary.BreakRotator` (`SceneComponent.RelativeRotation` (`/Game/RTS-Colombia/Blueprints/Player/RTS_CamaraPawn_BP.Sphere` (`/Game/RTS-Colombia/Blueprints/Player/RTS_PlayerController_BP.CameraPawnRef` (`self.PlayerControllerRef`))))))
  (`SceneComponent.K2_SetWorldRotation` (`self.BuildingStatusBar`) (`KismetMathLibrary.MakeRotator` _relativerotation_roll _relativerotation_pitch (+ _relativerotation_yaw 180.0)) false false)
  (return))

(fn `ReduceHealth`
  (params (Damage :type "Float (double-precision)"))
  (locals (DamageLocal :type "Float (double-precision)"))
  (set `local.DamageLocal` (* Damage 0.5))
  (set `self.CurrentHealth` (- (`self.CurrentHealth`) (`local.DamageLocal`)))
  (`self.UpdateBuildingHealth`)
  (if (< (`self.CurrentHealth`) 1.0)
    (set `self.CurrentHealth` 0.0))
  (return))

(fn `ReleaseAllOccupants`
  (for _array_element (`self.Occupants`)
    (`self.SetActorHiddenInGame` _array_element false)
    (set `/Game/RTS-Colombia/Unidades/RTS_UnidadMaster.IsHidden` false _array_element))
  (return))

(fn `ReleaseSingleOccupant`
  (params (Unit :type "/Game/RTS-Colombia/Unidades/RTS_UnidadMaster Object Reference"))
  (bind _occupants (`self.Occupants`))
  (`self.SetActorHiddenInGame` Unit false)
  (set `/Game/RTS-Colombia/Unidades/RTS_UnidadMaster.IsHidden` false Unit)
  (for (_array_element _array_index) _occupants
    (if (== _array_element Unit)
      (`KismetArrayLibrary.Array_Remove` _occupants _array_index)
      (message `/Game/RTS-Colombia/Blueprints/Library/RTS_OccupantiNFO.SetOccupantName` (`self.BuildingHUD`) (`self.Occupants`))
      (`/Game/RTS-Colombia/Blueprints/Widgets/BuildingInfo_HUD.UpdateOccupantList` (`self.BuildingHUD`))
      (return))))

(fn `SetArmorBarHidden`
  (`Widget.SetVisibility` (`/Game/RTS-Colombia/Blueprints/Widgets/W_DisplayStatus.ArmorProgBar` (cast `/Game/RTS-Colombia/Blueprints/Widgets/W_DisplayStatus` (`WidgetComponent.GetUserWidgetObject` (`self.BuildingStatusBar`)) :!pure true)) "Hidden")
  (return))

(fn `SetConstructionTIme`
  (params (ConstructionTimeRaw :type "Float (double-precision)"))
  (set `self.ConstructionTime` (* ConstructionTimeRaw 60.0))
  (return))

(fn `SetOccupantName`
  (params (Units :type "Array of /Game/RTS-Colombia/Unidades/RTS_UnidadMaster Object Reference (by ref)"))
  (returns (Success :type Boolean))
  (return false))

(fn `SetStatusBarHeight`
  (`SceneComponent.K2_SetRelativeLocation` (`self.BuildingStatusBar`) (`KismetMathLibrary.MakeVector` 0.0 0.0 (+ (.z (`.Max` (`StaticMeshComponent.GetLocalBounds` (`self.BuildingMesh`)))) 100.0)) false false)
  (return))

(fn `SetStatusBarHidden`
  (bind _buildingstatusbar (`self.BuildingStatusBar`))
  (`SceneComponent.SetHiddenInGame` _buildingstatusbar true true)
  (`SceneComponent.SetVisibility` _buildingstatusbar false true)
  (return))

(fn `SetStatusBarVIsible`
  (bind _buildingstatusbar (`self.BuildingStatusBar`))
  (`SceneComponent.SetHiddenInGame` _buildingstatusbar false true)
  (`SceneComponent.SetVisibility` _buildingstatusbar true true)
  (return))

(fn `UpdateBuildingHealth`
  (`ProgressBar.SetPercent` (`/Game/RTS-Colombia/Blueprints/Widgets/W_DisplayStatus.HealthProfBar` (cast `/Game/RTS-Colombia/Blueprints/Widgets/W_DisplayStatus` (`WidgetComponent.GetUserWidgetObject` (`self.BuildingStatusBar`)) :!pure true)) (/ (`self.CurrentHealth`) (`self.MaxHealth`)))
  (return))

(fn `UserConstructionScript`
  (`StaticMeshComponent.SetStaticMesh` (`self.BuildingMesh`) (`self.DisplayMesh`))
  (`BoxComponent.SetBoxExtent` (`self.EntryPoint`) (`.Max` (`StaticMeshComponent.GetLocalBounds` (`self.BuildingMesh`))) true)
  (if (`self.IsBuilt`)
    (`PrimitiveComponent.SetMaterial` (`self.BuildingMesh`) 0 null)
    (`self.SetStatusBarVIsible`)
    (`self.SetStatusBarHeight`)
    (else
      (`PrimitiveComponent.SetMaterial` (`self.BuildingMesh`) 0 "/Game/RTS-Colombia/Materiales/Etiquetas_SeleccionMovimiento/Construccion/Preview_M_Inst.Preview_M_Inst")
      (`self.SetStatusBarHidden`)
      (`self.SetStatusBarHeight`))))