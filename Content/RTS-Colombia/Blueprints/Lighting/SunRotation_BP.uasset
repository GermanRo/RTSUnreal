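; Blueprint actor that drives the day/night cycle by rotating a sun actor to match the game clock.
; On BeginPlay it caches the RTS game state.
; Every tick it converts the game state's GameTime from hours to seconds, scales it into a pitch angle offset by 90 degrees, and applies it to the sun.
; It then calls the sky sphere's sun direction update so the sky follows the light.
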(event `self.ReceiveBeginPlay`
  (set `self.GameStateRef` (cast `/Game/RTS-Colombia/Blueprints/GameSettings/RTS_GameState_BP` (`GameplayStatics.GetGameState`) :!pure true)))

(event `self.ReceiveTick`
  (params (DeltaSeconds :type "Float (single-precision)"))
  (`self.K2_SetActorRotation` (`self.SunRef`) (`KismetMathLibrary.MakeRotator` 0.0 (+ (* (* (`/Game/RTS-Colombia/Blueprints/GameSettings/RTS_GameState_BP.GameTime` (`self.GameStateRef`)) 3600.0) 0.004167) 90.0)) false)
  (`/Engine/EngineSky/BP_Sky_Sphere.UpdateSunDirection` (`self.SkySphereRef`)))

(fn `UserConstructionScript`)